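; Behavior tree task that makes a BP_Zombie perform a melee attack on the player.
; It plays an attack sound, lowers the zombie's roaming audio and plays the attack montage.
; On the montage notify, it applies random damage to the TargetActor if it overlaps the zombie's DamageCollision.
; Montage completion or interruption finishes the task as success or failure and restores the roaming volume.
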(event EventReceiveExecute
  (params (OwnerActor :type Actor%20Object%20Reference))
  (bind _asbp_zombie (Utilities|Casting|CastToBP_Zombie (Class|BTFunctionLibrary|GetBlackboardValueasObject (Utilities|Struct|MakeBlackboardKeySelector 0 "SelfActor" "/Script/AIModule.BlackboardKeyType_Object" 255 false))))
  (Audio|PlaySound2D "/Game/FPS_game/Characters/Male_Zombie/zombie_attack_sound.zombie_attack_sound" 1.0 1.0 0.0 0 0)
  (Audio|Components|Audio|SetVolumeMultiplier (Variables|/Game/FPS_game/Characters/BP_Zombie.BP_Zombie_C|GetAudioRoaming _asbp_zombie) 0.15 :!class /Script/Engine.AudioComponent)
  (Animation|Montage|PlayMontage (Variables|/Script/Engine.Character|GetMesh _asbp_zombie) "/Game/FPS_game/Characters/Male_Zombie/AM_Zombie.AM_Zombie"
    (:OnCompleted
      (AI|BehaviorTree|FinishExecute true)
      (Audio|Components|Audio|SetVolumeMultiplier (Variables|/Game/FPS_game/Characters/BP_Zombie.BP_Zombie_C|GetAudioRoaming _asbp_zombie) 1.0 :!class /Script/Engine.AudioComponent :!label _label))
    (:OnInterrupted
      (AI|BehaviorTree|FinishExecute false)
      (goto _label))
    (:OnNotifyBegin
      (bind _asbp_fpscharacter (Utilities|Casting|CastToBP_FPSCharacter (Class|BTFunctionLibrary|GetBlackboardValueasObject (Utilities|Struct|MakeBlackboardKeySelector 0 "TargetActor" "/Script/AIModule.BlackboardKeyType_Object" 255 false))))
      (if (Collision|IsOverlappingActor (Variables|/Game/FPS_game/Characters/BP_Zombie.BP_Zombie_C|GetDamageCollision _asbp_zombie) _asbp_fpscharacter :!class /Script/Engine.PrimitiveComponent)
        (Game|Damage|ApplyDamage _asbp_fpscharacter (Math|Random|RandomFloatinRange 15.0 25.0) 0 0)))))